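; BP_Target_+Time is a shootable target that extends the gameplay time limit when hit.
; When a FirstPersonProjectile begins overlapping its TargetCollision, it adds BonusTime to GameTimeLimit on BP_GameMode_Gameplay and plays a 2D confirmation sound.
; The handler leaves both target and projectile in place, with no guard against repeat hits.
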(event `self.TargetCollision.OnComponentBeginOverlap`
  (params (OverlappedComponent :type "PrimitiveComponent Object Reference") (OtherActor :type "Actor Object Reference") (OtherComp :type "PrimitiveComponent Object Reference") (OtherBodyIndex :type Integer) (bFromSweep :type Boolean) (SweepResult :type "HitResult Structure (by ref)"))
  ;[1 1 1] Add Time When Hit
  (cast `/Game/FirstPersonBP/Blueprints/FirstPersonProjectile` OtherActor)
  (bind _asbp_game_mode_gameplay (cast `/Game/MyContent/Blueprints/Framework/BP_GameMode_Gameplay` (`GameplayStatics.GetGameMode`)))
  (set `/Game/MyContent/Blueprints/Framework/BP_GameMode_Gameplay.GameTimeLimit` (+ (`/Game/MyContent/Blueprints/Framework/BP_GameMode_Gameplay.GameTimeLimit` _asbp_game_mode_gameplay) (`self.BonusTime`)) _asbp_game_mode_gameplay)
  (`GameplayStatics.PlaySound2D` "/Engine/VREditor/Sounds/VR_confirm_Cue.VR_confirm_Cue" 1.0 1.0 0.0 null null))

(fn `UserConstructionScript`
  (`parent.UserConstructionScript`))