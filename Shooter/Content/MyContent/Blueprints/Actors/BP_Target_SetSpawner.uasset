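; Trigger-driven spawner that places a set of five targets in the level when the first-person player enters its volume.
; A TriggerVolume overlap filtered to FirstPersonCharacter passes through a DoOnce, so the set spawns only once.
; A Sequence then starts five parallel Delays, each spawning its own configurable target class at a matching scene component's transform after a per-target delay.
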(event `self.TriggerVolume.OnComponentBeginOverlap`
  (params (OverlappedComponent :type "PrimitiveComponent Object Reference") (OtherActor :type "Actor Object Reference") (OtherComp :type "PrimitiveComponent Object Reference") (OtherBodyIndex :type Integer) (bFromSweep :type Boolean) (SweepResult :type "HitResult Structure (by ref)"))
  (cast `/Game/FirstPersonBP/Blueprints/FirstPersonCharacter` OtherActor)
  (`/Engine/EditorBlueprintResources/StandardMacros.DoOnce` false
    (:`Completed`
      (`|ExecutionSequence`
        (:`then_0`
          ;[1 1 1] Target 1
          (`KismetSystemLibrary.Delay` (`self.Target_01_Delay`))
          (`|SpawnActorFromClass` (`self.Target_01`) (`SceneComponent.K2_GetComponentToWorld` (`self.SpawnTarget_01`)) "Undefined" "OverrideRootScale" null null))
        (:`then_1`
          ;[1 1 1] Target 2
          (`KismetSystemLibrary.Delay` (`self.Target_02_Delay`))
          (`|SpawnActorFromClass` (`self.Target_02`) (`SceneComponent.K2_GetComponentToWorld` (`self.SpawnTarget_02`)) "Undefined" "OverrideRootScale" null null))
        (:`then_2`
          ;[1 1 1] Target 3
          (`KismetSystemLibrary.Delay` (`self.Target_03_Delay`))
          (`|SpawnActorFromClass` (`self.Target_03`) (`SceneComponent.K2_GetComponentToWorld` (`self.SpawnTarget_03`)) "Undefined" "OverrideRootScale" null null))
        (:`then_3`
          ;[1 1 1] Target 4
          (`KismetSystemLibrary.Delay` (`self.Target_04_Delay`))
          (`|SpawnActorFromClass` (`self.Target_04`) (`SceneComponent.K2_GetComponentToWorld` (`self.SpawnTarget_04`)) "Undefined" "OverrideRootScale" null null))
        (:`then_4`
          ;[1 1 1] Target 5
          (`KismetSystemLibrary.Delay` (`self.Target_05_Delay`))
          (`|SpawnActorFromClass` (`self.Target_05`) (`SceneComponent.K2_GetComponentToWorld` (`self.SpawnTarget_05`)) "Undefined" "OverrideRootScale" null null))))))

(fn `UserConstructionScript`)